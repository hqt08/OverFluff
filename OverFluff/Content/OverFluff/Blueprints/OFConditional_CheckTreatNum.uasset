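; OverFluff conditional that checks the word entries in the game state's TreatsArr and reports whether causality is maintained or broken.
; Execute casts the Instigator to OverFluffGameStateBP and branches on the array's length.
; Two entries maintain causality if they contain "Collect" and "Treats"; three break it only when starting "Three", "Collect", and otherwise maintain it.
; A failed cast or any other case defers to the parent's Execute.
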(fn `Execute`
  (params (Instigator :type "Actor Object Reference") (Other :type "Actor Object Reference"))
  (returns (`Casuality Maintained` :type Boolean) (`Casuality Broken` :type Boolean))
  (bind _asover_fluff_game_state_bp (cast `/Game/OverFluff/Project/OverFluffGameStateBP` Instigator)
    (:`then`
      (bind _treatsarr (`/Game/OverFluff/Project/OverFluffGameStateBP.TreatsArr` _asover_fluff_game_state_bp))
      (switch `int` (`KismetArrayLibrary.Array_Length` _treatsarr)
        (:`Default`
          _)
        (:`2`
          (if (and (`KismetArrayLibrary.Array_Contains` _treatsarr "Collect") (`KismetArrayLibrary.Array_Contains` _treatsarr "Treats"))
            (return true false)
            (else
              _)))
        (:`3`
          (if (and (`KismetStringLibrary.EqualEqual_StrStr` (`|GetArrayItem` _treatsarr) "Three") (`KismetStringLibrary.EqualEqual_StrStr` (`|GetArrayItem` _treatsarr 1) "Collect"))
            (return false true)
            (else
              (return true false))))))
    (:`CastFailed`
      _))
  ;[1 1 1] False fallback
  (bind (_casuality_maintained _casuality_broken) (`parent.Execute` Instigator Other))
  (return _casuality_maintained _casuality_broken))