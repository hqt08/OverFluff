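; Treat actor that players can spot and interact with by proximity, using two overlap radii.
; Entering the viewable radius shows a display widget and sets the OverFluffInteractible state to Viewable for that player controller; leaving hides it and resets to None.
; Overlapping the usable radius sets Interacting immediately and prints a pickup message, with no other pickup logic here.
; All overlap responses apply only to locally controlled OverFluff characters.
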(event `self.ViewableRadius.OnComponentBeginOverlap`
  (params (OverlappedComponent :type "PrimitiveComponent Object Reference") (OtherActor :type "Actor Object Reference") (OtherComp :type "PrimitiveComponent Object Reference") (OtherBodyIndex :type Integer) (bFromSweep :type Boolean) (SweepResult :type "HitResult Structure (by ref)"))
  (bind _asover_fluff_character (cast `OverFluffCharacter` OtherActor))
  (if (`Pawn.IsLocallyControlled` _asover_fluff_character)
    (`self.MakeViewable` true)
    (bind _asover_fluff_player_controller (cast `OverFluffPlayerController` (`Pawn.GetController` _asover_fluff_character)))
    (`/Engine/EditorBlueprintResources/StandardMacros.IsValid` (`self.GetComponentByClass` _asover_fluff_player_controller "/Script/OverFluff.OverFluffInteractionComponent")
      (:`Is Valid`
        (`OverFluffInteractibleComponent.ChangeInteractionState` (`self.OverFluffInteractible`) _asover_fluff_player_controller "Viewable")))))

(event `self.ViewableRadius.OnComponentEndOverlap`
  (params (OverlappedComponent :type "PrimitiveComponent Object Reference") (OtherActor :type "Actor Object Reference") (OtherComp :type "PrimitiveComponent Object Reference") (OtherBodyIndex :type Integer))
  (bind _asover_fluff_character (cast `OverFluffCharacter` OtherActor))
  (if (`Pawn.IsLocallyControlled` _asover_fluff_character)
    (`self.MakeViewable` false)
    (bind _asover_fluff_player_controller (cast `OverFluffPlayerController` (`Pawn.GetController` _asover_fluff_character)))
    (`OverFluffInteractibleComponent.ChangeInteractionState` (`self.OverFluffInteractible`) _asover_fluff_player_controller "None")))

(event `self.UsableRadius.OnComponentBeginOverlap`
  (params (OverlappedComponent :type "PrimitiveComponent Object Reference") (OtherActor :type "Actor Object Reference") (OtherComp :type "PrimitiveComponent Object Reference") (OtherBodyIndex :type Integer) (bFromSweep :type Boolean) (SweepResult :type "HitResult Structure (by ref)"))
  (bind _asover_fluff_character (cast `OverFluffCharacter` OtherActor))
  (if (`Pawn.IsLocallyControlled` _asover_fluff_character)
    (bind _asover_fluff_player_controller (cast `OverFluffPlayerController` (`Pawn.GetController` _asover_fluff_character)))
    (`OverFluffInteractibleComponent.ChangeInteractionState` (`self.OverFluffInteractible`) _asover_fluff_player_controller "Interacting")
    (`KismetSystemLibrary.PrintString` "Picked up treat")))

(event `self.ReceiveBeginPlay`)

(fn `MakeViewable`
  (params (bShow :type Boolean))
  (if bShow
    (`SceneComponent.SetVisibility` (`self.DisplayWidget`) true true)
    (else
      (`SceneComponent.SetVisibility` (`self.DisplayWidget`) false true))))

(fn `UserConstructionScript`)