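; Point-of-interest component that marks its owning actor on the player's minimap.
; On BeginPlay it registers the owner in the local OverFluff player controller's POI actor list.
; While Pending, Tick polls the main HUD until the minimap widget is valid, then adds the icon and clears the flag.
; Icons are skipped for locally controlled characters, so the local player is not marked as a POI.
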(event `Add POI Icon`
  (bind _ascharacter (cast `Character` (`self.GetOwner`))
    (:`then`
      (if (not (`Pawn.IsLocallyControlled` _ascharacter))
        (bind _minimapwidget (`self.GetMiniMapWidget` :!label _label))
        (`/Game/OverFluff/UI/MiniMapWidget.Add POI Event` _minimapwidget (`self.GetOwner`))))
    (:`CastFailed`
      (goto _label))))

(event `self.ReceiveBeginPlay`
  (bind _returnvalue (`GameplayStatics.GetPlayerController` 0))
  ;[1 1 1] Just a central local place to store the POIs
  (if (`Controller.IsLocalController` _returnvalue)
    (bind _asover_fluff_player_controller_bp (cast `/Game/OverFluff/Project/OverFluffPlayerControllerBP` _returnvalue)
      (:`then`
        (`KismetArrayLibrary.Array_Add` (`/Game/OverFluff/Project/OverFluffPlayerControllerBP.POI Actors` _asover_fluff_player_controller_bp) (`self.GetOwner`)))
      (:`CastFailed`
        (`KismetSystemLibrary.PrintString` "Failed to find player controller")))))

(event `self.ReceiveTick`
  (params (DeltaSeconds :type "Float (single-precision)"))
  (if (`self.bPending`)
    (cast `/Game/OverFluff/Project/OverFluffPlayerControllerBP` (`GameplayStatics.GetPlayerController` 0))
    (bind _minimapwidget (`self.GetMiniMapWidget`))
    (`/Engine/EditorBlueprintResources/StandardMacros.IsValid` _minimapwidget
      (:`Is Valid`
        (`self.Add POI Icon`)
        (set `self.bPending` false)))))

(fn `GetMiniMapWidget`
  (returns (MiniMapWidget :type "/Game/OverFluff/UI/MiniMapWidget Object Reference"))
  (bind _asmain_hud (cast `/Game/OverFluff/Project/MainHUD` (`PlayerController.GetHUD` (`GameplayStatics.GetPlayerController` 0))))
  (bind _mainhudwidget (`/Game/OverFluff/Project/MainHUD.MainHUDWidget` _asmain_hud))
  (`/Engine/EditorBlueprintResources/StandardMacros.IsValid` _mainhudwidget
    (:`Is Valid`
      (return (`/Game/OverFluff/UI/MainHUDWidget.MiniMapWidget` _mainhudwidget)))
    (:`Is Not Valid`
      (return null))))