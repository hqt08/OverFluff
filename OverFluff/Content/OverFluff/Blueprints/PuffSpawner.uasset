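; PuffSpawner is an actor that emits PuffBall actors at a timed interval until it reaches a set count.
; Tick accumulates delta time and, once it exceeds SpawnInterval, resets the timer and spawns a ball at the spawner's transform.
; Each new ball's Sphere component gets a fixed diagonal, mass-independent force in world X and Y to launch it.
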(event `self.ReceiveTick`
  (params (DeltaSeconds :type "Float (single-precision)"))
  (set `self.Time Interval` (+ (`self.Time Interval`) DeltaSeconds))
  (if (and (> (`self.Time Interval`) (`self.Spawn Interval`)) (< (`self.Number Spawned So Far`) (`self.Number To Spawn`)))
    (set `self.Time Interval` 0.0)
    (bind _returnvalue (`|SpawnActorFromClass` "/Game/OverFluff/Blueprints/PuffBall.PuffBall_C" (`self.GetTransform`) "Undefined" "OverrideRootScale" null null))
    (bind _result (`/Engine/EditorBlueprintResources/StandardMacros.IncrementInt` (`self.Number Spawned So Far`))
      (:`  `
        (set `self.Number Spawned So Far` _result)
        (`PrimitiveComponent.AddForce` (`/Game/OverFluff/Blueprints/PuffBall.Sphere` _returnvalue) (10000.0 10000.0 0.0) "None" true)))))

(fn `UserConstructionScript`)