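; Behavior tree service that detects targets for a follower AI to chase.
; Each tick it sphere-traces around the pawn for the desired object types, ignoring AI characters, then line-traces to each hit.
; A dot product against the head socket's right vector serves as the frontal check.
; Visible hits in front set TargetToFollow and TargetLocation on the blackboard; failed hits clear TargetToFollow, so the last hit decides.
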(event `self.ReceiveTick`
  (params (OwnerActor :type "Actor Object Reference") (DeltaSeconds :type "Float (single-precision)"))
  (bind _mesh (`Character.Mesh` (`self.AICharacterRef`)))
  (bind _returnvalue (`Actor.K2_GetActorLocation` (`Controller.K2_GetPawn` (`self.Follower_AI_Controller_Ref`))))
  (`/Engine/EditorBlueprintResources/StandardMacros.IsValid` (`self.Follower_AI_Controller_Ref`)
    (:`Is Valid`
      _)
    (:`Is Not Valid`
      (bind _asfollower_ai_controller (cast `/Game/OverFluff/Blueprints/AI_Test/Follower_AI_Controller` OwnerActor))
      (set `self.Follower_AI_Controller_Ref` _asfollower_ai_controller)))
  (bind _outactors (`GameplayStatics.GetAllActorsOfClass` "/Game/OverFluff/Blueprints/AI_Test/AI_Character.AI_Character_C"))
  (set `self.MyLocation` _returnvalue)
  (bind _outhits (`KismetSystemLibrary.SphereTraceMultiForObjects` _returnvalue (+ _returnvalue (0.0 0.0 15.0)) 1500.0 (`self.DesiredObjectTypes`) false _outactors))
  (for _array_element _outhits
    (bind (_bblockinghit _binitialoverlap _time _distance _location _impactpoint _normal _impactnormal _physmat _hitactor) (`GameplayStatics.BreakHitResult` _array_element))
    (bind _outhit (`KismetSystemLibrary.LineTraceSingle` (`self.MyLocation`) (`Actor.K2_GetActorLocation` _hitactor) "TraceTypeQuery2" false _outactors))
    (bind _ascharacter (cast `Character` (`Controller.K2_GetPawn` (`self.Follower_AI_Controller_Ref`))))
    (set `self.AICharacterRef` _ascharacter)
    (if (>= (`KismetMathLibrary.Dot_VectorVector` (- (`Actor.K2_GetActorLocation` _hitactor) (`SceneComponent.GetSocketLocation` _mesh "head")) (`KismetMathLibrary.GetRightVector` (`SceneComponent.GetSocketRotation` _mesh "head"))) 0.0)
      (bind (_bblockinghit_2 _binitialoverlap_2 _time_2 _distance_2 _location_2 _impactpoint_2 _normal_2 _impactnormal_2 _physmat_2 _hitactor_2) (`GameplayStatics.BreakHitResult` _outhit))
      (if (== _hitactor_2 _hitactor)
        (`BTFunctionLibrary.SetBlackboardValueAsObject` (`self.TargetToFollow`) _hitactor_2)
        (`BTFunctionLibrary.SetBlackboardValueAsVector` (`self.TargetLocation`) (`Actor.K2_GetActorLocation` _hitactor_2))
        (else
          (`BTFunctionLibrary.SetBlackboardValueAsObject` (`self.TargetToFollow`) :!label _label)))
      (else
        (goto _label)))))