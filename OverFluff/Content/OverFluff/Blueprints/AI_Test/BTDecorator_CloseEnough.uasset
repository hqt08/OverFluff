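; Behavior Tree decorator for the follower AI that gates a branch on the distance between the follower and its target.
; It casts the owner to Follower_AI_Controller, then measures from the controlled pawn to the actor in the TargetToFollow blackboard key.
; Despite the CloseEnough name, it passes when that distance is at or beyond AcceptableDist, meaning the follower is too far away.
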(fn `PerformConditionCheck`
  (params (OwnerActor :type "Actor Object Reference"))
  (returns (ReturnValue :type Boolean))
  (bind _asfollower_ai_controller (cast `/Game/OverFluff/Blueprints/AI_Test/Follower_AI_Controller` OwnerActor))
  (set `self.AI_Controller_Ref` _asfollower_ai_controller)
  (return (>= (`KismetMathLibrary.VSize` (- (`Actor.K2_GetActorLocation` (`BTFunctionLibrary.GetBlackboardValueAsActor` (`self.TargetToFollow`))) (`Actor.K2_GetActorLocation` (`Controller.K2_GetPawn` (`self.AI_Controller_Ref`))))) (`self.AcceptableDist`))))