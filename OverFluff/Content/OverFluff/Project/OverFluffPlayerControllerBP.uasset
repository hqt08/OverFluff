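; OverFluff player controller Blueprint that provides events for hosting and finding online sessions.
; Both SERVER events cast the game instance to OverFluffGameInstanceBP and pass it LAN session requests, printing an error if the cast fails.
; The search returns through a completion event that prints each found session's server name.
; An unconnected FindSessions node chain remains in the graph but never runs.
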(event `SERVER_HostSession`
  (bind _asover_fluff_game_instance_bp (cast `/Game/OverFluff/Project/OverFluffGameInstanceBP` (`GameplayStatics.GetGameInstance`))
    (:`then`
      (`OverFluffGameInstance.RequestHostSession` _asover_fluff_game_instance_bp self "Test 1" true true 5))
    (:`CastFailed`
      (`KismetSystemLibrary.PrintString` "Could not find GameInstance" :!label _label))))

(event `SERVER_FindSessions`
  (bind _asover_fluff_game_instance_bp (cast `/Game/OverFluff/Project/OverFluffGameInstanceBP` (`GameplayStatics.GetGameInstance`))
    (:`then`
      (`OverFluffGameInstance.RequestFindSessions` _asover_fluff_game_instance_bp self true true (delegate `OnSessionSearchCompleteEvent`)))
    (:`CastFailed`
      (goto _label))))

(event `OnSessionSearchCompleteEvent`
  (params (Results :type "Array of BlueprintSessionResult Structure (by ref)"))
  (for _array_element Results
    (`KismetSystemLibrary.PrintString` (`KismetStringLibrary.Concat_StrStr` "Session Name: " (`FindSessionsCallbackProxy.GetServerName` _array_element)))))

(fn `UserConstructionScript`)