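; OverFluff game state that tracks a tally of treats and reports whether causality is maintained or broken.
; Adding to the tally runs a newly constructed OFConditional_CheckTreatNum, whose result triggers a multicast that calls the matching maintained or broken delegate.
; A separate multicast forwards an interactible actor to the local player character's client finish event for HUD updates, and a debug function prints the tally.
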(event `MULTICAST_OnCasualityMaintained`
  (`self.OnCasualityMaintainedDelegate`))

(event `MULTICAST_OnCasualityBroken`
  (`self.OnCasualityBrokenDelegate`))

(event `MULTICAST_HUDUpdate`
  (params (`Interactible Actor` :type "Actor Object Reference"))
  (bind _asover_fluff_character_bp (cast `/Game/OverFluff/Project/OverFluffCharacterBP` (`GameplayStatics.GetPlayerPawn` 0)))
  (`/Game/OverFluff/Project/OverFluffCharacterBP.CLIENT_OnFinished` _asover_fluff_character_bp `Interactible Actor`))

(fn `AddToTreatTally`
  (params (Word :type String))
  (`KismetArrayLibrary.Array_Add` (`self.TreatsArr`) Word)
  (`self.CheckCausality`))

(fn `CheckCausality`
  (bind _returnvalue (`|GenericCreateObject` "/Game/OverFluff/Blueprints/OFConditional_CheckTreatNum.OFConditional_CheckTreatNum_C" self))
  (`/Engine/EditorBlueprintResources/StandardMacros.IsValid` _returnvalue
    (:`Is Valid`
      (bind (_casuality_maintained _casuality_broken) (`/Game/OverFluff/Blueprints/OFConditional.Execute` _returnvalue self null))
      (if _casuality_maintained
        (`self.MULTICAST_OnCasualityMaintained`)
        (elif _casuality_broken
          (`self.MULTICAST_OnCasualityBroken`))))
    (:`Is Not Valid`
      (`KismetSystemLibrary.PrintString` "Conditional not valid"))))

(fn `Debug_PrintTreatsArr`
  (bind _treatsarr (`self.TreatsArr`))
  (for _array_element _treatsarr
    (`KismetSystemLibrary.PrintString` _array_element true true (struct :`R` 1.0 :`B` 0.011349 :`A` 1.0)))
  (`KismetSystemLibrary.PrintString` (`KismetStringLibrary.Conv_IntToString` (`KismetArrayLibrary.Array_Length` _treatsarr)) true true (struct :`R` 1.0 :`G` 0.101995 :`A` 1.0)))

(fn `UserConstructionScript`)